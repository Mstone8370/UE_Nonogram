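; Blueprint function helpers that build image paths for game boards from a folder name and board name.
; ToAssetPath composes the Texture2D object path of a board's T_-prefixed texture under Textures/BoardCleared.
; ToSavedPath composes a .bmp path inside the project Saved directory's img/InProgress folder, via GetSavedImgDir, with an optional file:/// scheme prefix.
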(fn ToAssetPath
  (params (FolderName :type Name) (BoardName :type Name))
  (bind _returnvalue (Utilities|String|ToString(Name) BoardName))
  (bind _returnvalue_2 (Utilities|String|Append "T_" _returnvalue))
  (return (Utilities|String|Append "/Script/Engine.Texture2D'/Game/_Game/Textures/BoardCleared/" (Utilities|String|ToString(Name) FolderName) "/" _returnvalue_2 "." _returnvalue_2 "'")))

(fn ToSavedPath
  (params (FolderName :type Name) (BoardName :type Name) (bIncludeFileScheme :type Boolean))
  (return (Utilities|String|Append (Utilities|String|SelectString "file:///" "" bIncludeFileScheme) (CallFunction|GetSavedImgDir (LocalVariables|Get__WorldContext)) (Utilities|String|ToString(Name) FolderName) "/" (Utilities|String|ToString(Name) BoardName) ".bmp")))

(fn GetSavedImgDir
  (return (Utilities|String|Append (Class|KismetSystemLibrary|GetProjectSavedDirectory) "img/InProgress/")))