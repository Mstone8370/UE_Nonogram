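; Option item that wraps an OptionStruct and tracks a pending value for one option.
; The bool, int and float setters each check the option type, store the new value and set OptionChanged when it differs from the struct's value.
; The byte setter is an empty stub.
; Test prints the display text and holds unconnected debug logic that would list enum names by EnumType.
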(fn Test
  (Development|PrintString 0 (Utilities|String|ToString(Text) (.DisplayText (Utilities|Struct|BreakST_Option (Variables|Default|GetOptionStruct))))))

(fn SetNewBoolVal
  (params (Val :type Boolean))
  (bind _optionstruct (Variables|Default|GetOptionStruct))
  (bind (_displaytext _bisenabled _optiontype _boolval) (Utilities|Struct|BreakST_Option _optionstruct))
  (if (Utilities|Enum|Equal(Enum) "NewEnumerator0" _optiontype)
    (bind _output_get (Variables|Default|SetNewBoolVal Val))
    (Variables|Default|SetbOptionChanged (!= _output_get _boolval))))

(fn SetNewIntVal
  (params (Val :type Integer))
  (bind _optionstruct (Variables|Default|GetOptionStruct))
  (bind (_displaytext _bisenabled _optiontype _boolval _intval) (Utilities|Struct|BreakST_Option _optionstruct))
  (if (Utilities|Enum|Equal(Enum) "NewEnumerator1" _optiontype)
    (bind _output_get (Variables|Default|SetNewIntVal Val))
    (Variables|Default|SetbOptionChanged (!= _output_get _intval))))

(fn SetNewFloatVal
  (params (Val :type Float%20%28double-precision%29))
  (bind _optionstruct (Variables|Default|GetOptionStruct))
  (bind (_displaytext _bisenabled _optiontype _boolval _intval _floatval) (Utilities|Struct|BreakST_Option _optionstruct))
  (if (Utilities|Enum|Equal(Enum) "NewEnumerator2" _optiontype)
    (bind _output_get (Variables|Default|SetNewFloatVal Val))
    (Variables|Default|SetbOptionChanged (!= _output_get _floatval))))

(fn SetNewByteVal)