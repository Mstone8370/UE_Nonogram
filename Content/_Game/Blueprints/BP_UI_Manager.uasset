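; UI manager for a nonogram game that handles screen navigation, from menus to play, and user puzzle uploads.
; An enum stack tracks screens; Show functions reuse most widgets, in a shared base or the viewport, and CloseTopWidget pops and re-shows the previous one.
; Uploads in Make mode first request server validation through the game mode: one solution opens the upload widget, otherwise failure is shown and any ambiguous filled cells flagged.
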(event Custom|OnUploadButtonPressed
  (bind _ui_stack (Variables|Default|GetUI_Stack))
  (bind _gamemode_ref (Variables|Default|GetGameMode_Ref))
  (bind _boardmanager_ref (Variables|/Script/Nonogram.NonogramGameModeBase|GetBoardManager_Ref _gamemode_ref))
  (if (Math|Boolean|ANDBoolean (Utilities|Enum|Equal(Enum) (Class|BoardManager|GetBoardMode _boardmanager_ref) "EBM_Make") (Utilities|Enum|Equal(Enum) "NewEnumerator2" (Utilities|Array|Get(acopy) _ui_stack (Utilities|Array|LastIndex _ui_stack))) (> (Class|BoardManager|GetInfoCount _boardmanager_ref) 0))
    (Utilities|FlowControl|Sequence
      (:then_2
        (bind _gamemode_ref_2 (Variables|Default|GetGameMode_Ref)
          (:then
            (EventDispatchers|BindEventtoValidationResponseReceived _gamemode_ref_2 (EventDispatchers|CreateEvent :!event Custom|OnValidationResponseRecived))
            (Class|NonogramGameModeBase|RequestValidation _gamemode_ref_2 (Class|BoardManager|GetEncodedInfo _boardmanager_ref))
            (bind _returnvalue (UserInterface|CreateWidget "/Game/_Game/UI/UserPuzzle/WBP_ServerResponseWait.WBP_ServerResponseWait_C"))
            (bind _output_get (Variables|Widget_Ref|SetWBP_ServerResponseWait _returnvalue))
            (UserInterface|Viewport|AddtoViewport _output_get 0))
          (:else))))))

(event Custom|OnUserPuzzleUploadDone
  (CallFunction|CloseTopWidget)
  (Utilities|FlowControl|Sequence
    (:then_0
      (bind _wbp_userboardlist (Variables|Widget_Ref|GetWBP_UserBoardList)
        (:then
          (Default|RefreshList _wbp_userboardlist))
        (:else)))
    (:then_1
      (bind _returnvalue (UserInterface|CreateWidget "/Game/_Game/UI/UserPuzzle/WBP_UserPuzzleUploadDoneMessage.WBP_UserPuzzleUploadDoneMessage_C"))
      (Default|AddOverlayContent (Variables|Widget_Ref|GetWBP_Base) _returnvalue))))

(event Custom|OnUserPuzzleUploadFailed
  (Development|PrintString "Puzzle upload Failed" true true "(R=1.000000,G=0.000000,B=0.000000,A=1.000000)" 5.0))

(event Custom|OnValidationResponseRecived
  (params (bSuccess :type Boolean) (Body :type String))
  (Utilities|FlowControl|Sequence
    (:then_0
      (if bSuccess
        (bind _wbp_serverresponsewait (Variables|Widget_Ref|GetWBP_ServerResponseWait)
          (:then
            (Widget|RemovefromParent _wbp_serverresponsewait)
            (bind _outjsonobject (Class|JsonBlueprintFunctionLibrary|FromString Body))
            (CallFunction|ShowValidationResult _outjsonobject))
          (:else))
        (else
          (Development|PrintString "Request Failed")
          (bind _wbp_serverresponsewait_2 (Variables|Widget_Ref|GetWBP_ServerResponseWait)
            (:then
              (Widget|RemovefromParent _wbp_serverresponsewait_2))
            (:else)))))
    (:then_1
      (bind _gamemode_ref (Variables|Default|GetGameMode_Ref)
        (:then
          (EventDispatchers|UnbindEventfromValidationResponseReceived _gamemode_ref (EventDispatchers|CreateEvent :!event Custom|OnValidationResponseRecived)))
        (:else)))))

(event EventBeginPlay
  (CallFunction|Init))

(event EventTick
  (params (DeltaSeconds :type Float%20%28single-precision%29)))

(fn Init
  (Utilities|FlowControl|Sequence
    (:then_0
      (Utilities|Array|Clear (Variables|Default|GetUI_Stack))
      (bind _asbp_nono_gram_gmb (Utilities|Casting|CastToBP_NonoGramGMB (Game|GetGameMode)))
      (Variables|Default|SetGameMode_Ref _asbp_nono_gram_gmb))
    (:then_2
      (CallFunction|ShowMain))))

(fn Push
  (params (NewUI :type E_UIState%20Enum :default "NewEnumerator3"))
  (Utilities|Array|Add (Variables|Default|GetUI_Stack) NewUI))

(fn Pop
  (bind _ui_stack (Variables|Default|GetUI_Stack))
  (bind _returnvalue (Utilities|Array|LastIndex _ui_stack))
  (LocalVariables|SetRet (Utilities|Array|Get(acopy) _ui_stack _returnvalue))
  (Utilities|Array|RemoveIndex (Variables|Default|GetUI_Stack) _returnvalue)
  (return (LocalVariables|GetRet)))

(fn CloseTopWidget
  (bind _wbp_play (Variables|Widget_Ref|GetWBP_Play))
  (Utilities|FlowControl|Sequence
    (:then_0
      (bind _item (CallFunction|Pop))
      (Widget|RemovefromParent (Utilities|Select :Index _item :NewEnumerator3 0 :NewEnumerator0 (Variables|Widget_Ref|GetWBP_Main) :NewEnumerator5 (Variables|Widget_Ref|GetWBP_FolderSelect) :NewEnumerator1 (Variables|Widget_Ref|GetWBP_BoardSelect) :NewEnumerator8 (Variables|Widget_Ref|GetWBP_UserBoardList) :NewEnumerator2 _wbp_play :NewEnumerator4 _wbp_play :NewEnumerator6 (Variables|Widget_Ref|GetWBP_Completed) :NewEnumerator7 (Variables|Widget_Ref|GetWBP_Settings) :NewEnumerator9 (Variables|Widget_Ref|GetWBP_BoardSizeSelect)))
      (switch Utilities|FlowControl|Switch|SwitchonE_UIState _item
        (:NewEnumerator3
          (Development|PrintString "What?"))
        (:NewEnumerator0
          (Development|PrintString "Quit")
          (Game|QuitGame 0 "Quit" false))
        (:NewEnumerator5
          (Widget|RemovefromParent (Variables|Widget_Ref|GetWBP_Base) :!label _label))
        (:NewEnumerator8
          (Default|Clear (Variables|Widget_Ref|GetWBP_UserBoardList))
          (goto _label))
        (:NewEnumerator2
          (Default|EmptyBoard (Variables|Default|GetGameMode_Ref) :!label _label_2))
        (:NewEnumerator6
          (Widget|RemovefromParent (Variables|Widget_Ref|GetWBP_Play))
          (CallFunction|Pop)
          (goto _label_2))
        (:NewEnumerator7
          (return))))
    (:then_1
      (if (Utilities|Array|IsNotEmpty (Variables|Default|GetUI_Stack))
        (bind _item_2 (CallFunction|Pop))
        (switch Utilities|FlowControl|Switch|SwitchonE_UIState _item_2
          (:NewEnumerator0
            (CallFunction|ShowMain))
          (:NewEnumerator5
            (CallFunction|ShowFolderSelect))
          (:NewEnumerator1
            (CallFunction|ShowBoardSelect (Variables|Default|GetCurrentFolder)))
          (:NewEnumerator8
            (CallFunction|ShowUserBoardList)))
        (else
          (Development|PrintString "What?"))))))

(fn CheckBaseUI
  (Variables|Widget_Ref|GetWBP_Base
    (:then
      (if (UserInterface|Viewport|IsinViewport (Variables|Widget_Ref|GetWBP_Base))
        _
        (else
          (UserInterface|Viewport|AddtoViewport (stale _output_get) 0 :!label _label))))
    (:else
      (bind _returnvalue (UserInterface|CreateWidget "/Game/_Game/UI/WBP_Base.WBP_Base_C"))
      (bind _output_get (Variables|Widget_Ref|SetWBP_Base _returnvalue))
      (goto _label)))
  (Default|SetUploadButtonVisibility (Variables|Widget_Ref|GetWBP_Base) "Collapsed")
  (Default|SetCreateButtonVisibility (Variables|Widget_Ref|GetWBP_Base) "Collapsed"))

(fn ShowMain
  (CallFunction|Push "NewEnumerator0")
  (Variables|Widget_Ref|GetWBP_Main
    (:then)
    (:else
      (bind _returnvalue (UserInterface|CreateWidget "/Game/_Game/UI/WBP_Main.WBP_Main_C"))
      (Variables|Widget_Ref|SetWBP_Main _returnvalue)
      (UserInterface|Viewport|AddtoViewport (Variables|Widget_Ref|GetWBP_Main) 0))))

(fn ShowFolderSelect
  (CallFunction|Push "NewEnumerator5")
  (Utilities|FlowControl|Sequence
    (:then_0
      (CallFunction|CheckBaseUI))
    (:then_1
      (Variables|Widget_Ref|GetWBP_FolderSelect
        (:then
          _)
        (:else
          (bind _returnvalue (UserInterface|CreateWidget "/Game/_Game/UI/WBP_FolderSelect.WBP_FolderSelect_C"))
          (Variables|Widget_Ref|SetWBP_FolderSelect _returnvalue)))
      (Default|SetContent (Variables|Widget_Ref|GetWBP_Base) (Variables|Widget_Ref|GetWBP_FolderSelect)))))

(fn ShowBoardSelect
  (params (FolderName :type Name))
  (CallFunction|Push "NewEnumerator1")
  (Variables|Default|SetCurrentFolder FolderName)
  (Utilities|FlowControl|Sequence
    (:then_0
      (CallFunction|CheckBaseUI))
    (:then_1
      (bind _wbp_boardselect (Variables|Widget_Ref|GetWBP_BoardSelect)
        (:then
          (Default|ShowNewFolder _wbp_boardselect (Variables|Default|GetCurrentFolder)))
        (:else
          (bind _returnvalue (UserInterface|CreateWidget "/Game/_Game/UI/WBP_BoardSelect.WBP_BoardSelect_C" 0 (Variables|Default|GetCurrentFolder)))
          (Variables|Widget_Ref|SetWBP_BoardSelect _returnvalue)))
      (Default|SetContent (Variables|Widget_Ref|GetWBP_Base) (Variables|Widget_Ref|GetWBP_BoardSelect)))))

(fn ShowPlay
  (params (BoardInfo :type Board%20Info%20Structure) (BoardMode :type EBoardMode%20Enum :default "EBM_Play"))
  (CallFunction|Push "NewEnumerator2")
  (Utilities|FlowControl|Sequence
    (:then_0
      (CallFunction|CheckBaseUI)
      (if (Utilities|Enum|Equal(Enum) "EBM_Make" BoardMode)
        (Default|SetUploadButtonVisibility (Variables|Widget_Ref|GetWBP_Base) "SelfHitTestInvisible")))
    (:then_1
      (Variables|Widget_Ref|GetWBP_Play
        (:then
          _)
        (:else
          (bind _returnvalue (UserInterface|CreateWidget "/Game/_Game/UI/Board/WBP_Play.WBP_Play_C"))
          (Variables|Widget_Ref|SetWBP_Play _returnvalue)))
      (Default|SetBoardInfo (Variables|Widget_Ref|GetWBP_Play) BoardInfo BoardMode)
      (Default|SetContent (Variables|Widget_Ref|GetWBP_Base) (Variables|Widget_Ref|GetWBP_Play)))))

(fn ShowBoardClear
  (params (PlayTimeMinutes :type Integer) (PlayTimeSeconds :type Integer) (Texture :type Texture%202D%20Object%20Reference) (TextureDynamic :type Texture%202D%20Dynamic%20Object%20Reference) (bIsUserPuzzle :type Boolean) (BoardDisplayName :type Text))
  (CallFunction|Push "NewEnumerator6")
  (Utilities|FlowControl|Sequence
    (:then_0
      (bind _returnvalue (UserInterface|CreateWidget "/Game/_Game/UI/WBP_Completed.WBP_Completed_C" 0 BoardDisplayName (Utilities|Text|ToText(String) (Utilities|String|Append "시간: " (Utilities|String|ToString(Integer) PlayTimeMinutes) " 분 " (Utilities|String|ToString(Integer) PlayTimeSeconds) " 초"))))
      (Variables|Widget_Ref|SetWBP_Completed _returnvalue)
      (if bIsUserPuzzle
        (Default|SetBoardImageTextureDynamic (Variables|Widget_Ref|GetWBP_Completed) TextureDynamic)
        (else
          (Default|SetBoardImageTexture (Variables|Widget_Ref|GetWBP_Completed) Texture)))
      (UserInterface|Viewport|AddtoViewport (Variables|Widget_Ref|GetWBP_Completed) 0))))

(fn ShowSetting
  (CallFunction|Push "NewEnumerator7")
  (Variables|Widget_Ref|GetWBP_Settings
    (:then
      _)
    (:else
      (bind _returnvalue (UserInterface|CreateWidget "/Game/_Game/UI/Setting/WBP_Setting.WBP_Setting_C"))
      (Variables|Widget_Ref|SetWBP_Settings _returnvalue)))
  (UserInterface|Viewport|AddtoViewport (Variables|Widget_Ref|GetWBP_Settings) 0))

(fn ShowUserBoardList
  (CallFunction|Push "NewEnumerator8")
  (Utilities|FlowControl|Sequence
    (:then_0
      (CallFunction|CheckBaseUI)
      (Default|SetCreateButtonVisibility (Variables|Widget_Ref|GetWBP_Base) "SelfHitTestInvisible"))
    (:then_1
      (Variables|Widget_Ref|GetWBP_UserBoardList
        (:then
          _)
        (:else
          (bind _returnvalue (UserInterface|CreateWidget "/Game/_Game/UI/UserPuzzle/WBP_UserBoardList.WBP_UserBoardList_C"))
          (Variables|Widget_Ref|SetWBP_UserBoardList _returnvalue)))
      (Default|SetContent (Variables|Widget_Ref|GetWBP_Base) (Variables|Widget_Ref|GetWBP_UserBoardList)))))

(fn ShowPuzzleSizeSelect
  (CallFunction|Push "NewEnumerator9")
  (Variables|Widget_Ref|GetWBP_BoardSizeSelect
    (:then
      _)
    (:else
      (bind _returnvalue (UserInterface|CreateWidget "/Game/_Game/UI/WBP_BoardSizeSelect.WBP_BoardSizeSelect_C"))
      (Variables|Widget_Ref|SetWBP_BoardSizeSelect _returnvalue)))
  (UserInterface|Viewport|AddtoViewport (Variables|Widget_Ref|GetWBP_BoardSizeSelect) 0))

(fn ShowValidationResult
  (params (JSON :type Json%20Object%20Wrapper%20Structure))
  (bind _outvalue (|GetJsonField JSON "num"))
  (switch int _outvalue
    (:Default
      (bind _outvalue_2 (|GetJsonField JSON "ambiguous"))
      (for _array_element _outvalue_2
        (bind _wbp_cell (Default|GetCellWidgetat (Variables|/Game/_Game/UI/Board/WBP_Play.WBP_Play_C|GetWBP_Board (Variables|Widget_Ref|GetWBP_Play)) (Math|Conversions|ToInteger(Byte) (Utilities|Array|Get(acopy) (Utilities|String|ParseIntoArray _array_element "|"))) (Math|Conversions|ToInteger(Byte) (Utilities|Array|Get(acopy) (Utilities|String|ParseIntoArray _array_element "|") 1))))
        (if (Utilities|Enum|Equal(Enum) "ECS_Filled" (Variables|/Game/_Game/UI/Board/WBP_Cell.WBP_Cell_C|GetCellState _wbp_cell))
          (Default|ShowWarning _wbp_cell)))
      (bind _returnvalue (UserInterface|CreateWidget "/Game/_Game/UI/UserPuzzle/WBP_ValidationFailed.WBP_ValidationFailed_C" 0 _outvalue :!label _label))
      (UserInterface|Viewport|AddtoViewport _returnvalue 0))
    (:0
      (goto _label))
    (:1
      (bind _returnvalue_2 (UserInterface|CreateWidget "/Game/_Game/UI/UserPuzzle/WBP_UploadUserBoard.WBP_UploadUserBoard_C" 0 (Class|BoardManager|GetBoard (Variables|/Script/Nonogram.NonogramGameModeBase|GetBoardManager_Ref (Variables|Default|GetGameMode_Ref)))))
      (EventDispatchers|BindEventtoUploadDone _returnvalue_2 (EventDispatchers|CreateEvent :!event Custom|OnUserPuzzleUploadDone))
      (EventDispatchers|BindEventtoUploadFailed _returnvalue_2 (EventDispatchers|CreateEvent :!event Custom|OnUserPuzzleUploadFailed))
      (UserInterface|Viewport|AddtoViewport _returnvalue_2 0))))

(fn DEBUGSHOWUISTACK
  (for _array_element (Variables|Default|GetUI_Stack)
    (Development|PrintString (Utilities|String|EnumtoString _array_element) true false "(R=0.000000,G=0.660000,B=1.000000,A=1.000000)" 0.0)))

(fn OnPuzzleProgressResetted
  (Utilities|FlowControl|Sequence
    (:then_0
      (bind _wbp_boardselect (Variables|Widget_Ref|GetWBP_BoardSelect)
        (:then
          (Default|ShowNewFolder _wbp_boardselect (Variables|Default|GetCurrentFolder)))
        (:else)))
    (:then_1
      (bind _wbp_userboardlist (Variables|Widget_Ref|GetWBP_UserBoardList)
        (:then
          (Default|RefreshList _wbp_userboardlist))
        (:else)))))