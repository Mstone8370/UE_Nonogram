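; Player controller, apparently for a nonogram puzzle game, that sets up a free mouse cursor and Enhanced Input.
; BeginPlay disables viewport mouse capture, shows the cursor and adds the IMC_Back mapping context.
; IA_Key only prints its value, and its likely context IMC_Key is added only in unconnected nodes.
; Other unconnected leftovers include UI-only input mode and cell-click and back-button calls to BP_NonoGramGMB.
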(event Input|EnhancedActionEvents|EnhancedInputActionIA_Click
  (params (ActionValue :type Boolean) (ElapsedSeconds :type Float%20%28double-precision%29) (TriggeredSeconds :type Float%20%28double-precision%29) (InputAction :type Input%20Action%20Object%20Reference :default "/Game/_Game/Inputs/IA/IA_Click.IA_Click")))

(event Input|EnhancedActionEvents|EnhancedInputActionIA_Key
  (params (ActionValue :type Vector%202D%20Structure) (ElapsedSeconds :type Float%20%28double-precision%29) (TriggeredSeconds :type Float%20%28double-precision%29) (InputAction :type Input%20Action%20Object%20Reference :default "/Game/_Game/Inputs/IA/IA_Key.IA_Key"))
  (:Triggered
    (Development|PrintString (Utilities|String|ToString(Vector2d) ActionValue))))

(event Input|EnhancedActionEvents|EnhancedInputActionIA_Back
  (params (ActionValue :type Boolean) (ElapsedSeconds :type Float%20%28double-precision%29) (TriggeredSeconds :type Float%20%28double-precision%29) (InputAction :type Input%20Action%20Object%20Reference :default "/Game/_Game/Inputs/IA/IA_Back.IA_Back")))

(event EventBeginPlay
  (Class|GameplayStatics|SetViewportMouseCaptureMode "NoCapture")
  (Variables|Default|SetbShowMouseCursor true)
  (Input|AddMappingContext (PlayerController|LocalPlayerSubsystems|GetEnhancedInputLocalPlayerSubsystem) "/Game/_Game/Inputs/IMC/IMC_Back.IMC_Back" 1 "(bIgnoreAllPressedKeysUntilRelease=True,bForceImmediately=False)"))

(event EventTick
  (params (DeltaSeconds :type Float%20%28single-precision%29)))

(event Input|KeyboardEvents|AndroidBack
  (params (Key :type Key%20Structure :default "None")))

(fn ConstructionScript)