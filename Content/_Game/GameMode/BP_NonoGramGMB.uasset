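; Game mode for a nonogram puzzle game, linking the board manager, UI manager and game instance for play, user puzzles and puzzle making.
; BeginPlay constructs the manager, logger, image maker and UI.
; Cell press, hover and release become straight-line drag selections with crosshair previews, sent to the board manager as batched clicks.
; It saves and restores progress and play time per board, records completion, and can wipe all progress and saved images.
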(event Custom|OnCellReleasedEvent
  (params (RowIdx :type Integer) (ColIdx :type Integer))
  ;[1 1 1] Input related event
  (if (Variables|UserInteraction|GetMousePressed)
    (Variables|UserInteraction|SetReleasedCell (select (and (>= RowIdx 0) (>= ColIdx 0)) (Utilities|Struct|MakeST_Coord ColIdx RowIdx) (Variables|UserInteraction|GetHoveringCell)))
    (CallFunction|StopPreviewCells)
    (CallFunction|ClickMultipleCell)
    (Variables|UserInteraction|SetMousePressed false)
    (if (Variables|UserInteraction|GetIsMobilePlatform)
      (CallFunction|StopPreviewCrossingCells))))

(event Custom|OnBackButtonClicked
  (Default|CloseTopWidget (Variables|Default|GetUI_Manager)))

(event Custom|OnPuzzleMakerStarted
  (params (RowSize :type Integer) (ColSize :type Integer))
  (bind _boardinfo (CallFunction|GetBoardMakerInfo RowSize ColSize))
  (bind _ui_manager (Variables|Default|GetUI_Manager)
    (:then
      (Default|ShowPlay _ui_manager _boardinfo "EBM_Make"))
    (:else)))

(event Custom|OnBoardSelected
  (params (FolderName :type Name) (BoardName :type Name) (BoardDisplayName :type Text) (PuzzleImage :type Texture%202D%20Object%20Reference))
  (CallFunction|LoadBoard FolderName BoardName BoardDisplayName)
  (Variables|Default|SetbIsUserPuzzle false)
  (Variables|Default|SetCurrentBoardTexture PuzzleImage))

(event Custom|ResetBoard
  (bind _boardmanager_ref (Variables|Default|GetBoardManager_Ref)
    (:then
      (Class|BoardManager|ResetBoard _boardmanager_ref))
    (:else)))

(event Custom|OnCellHoveredEvent
  (params (RowIdx :type Integer) (ColIdx :type Integer))
  ;[1 1 1] Input related event
  (if (and (>= RowIdx 0) (>= ColIdx 0))
    (Variables|UserInteraction|SetHoveringCell (Utilities|Struct|MakeST_Coord ColIdx RowIdx))
    (CallFunction|PreviewCrossingCells)
    (if (Variables|UserInteraction|GetMousePressed)
      (CallFunction|PreviewCells))
    (else
      (CallFunction|StopPreviewCrossingCells))))

(event Custom|OnBoardCompleteEvent
  (bind (_time _minute _second) (CallFunction|GetPlayTime))
  (bind _currentfoldername (Variables|Default|GetCurrentFolderName))
  (bind _currentboardname (Variables|Default|GetCurrentBoardName))
  (bind _path (CallFunction|ToSavedPath _currentfoldername _currentboardname false))
  (bind _ui_manager (Variables|Default|GetUI_Manager)
    (:then
      (Default|ShowBoardClear _ui_manager _minute _second (Variables|Default|GetCurrentBoardTexture) (Variables|Default|GetCurrentBoardTextureDynamic) (Variables|Default|GetbIsUserPuzzle) (Variables|Default|GetCurrentBoardDisplayName))
      (bind _gi_ref (Variables|Default|GetGI_Ref)
        (:then
          (bind (_found _boardstate) (Default|GetBoardState _gi_ref (Variables|Default|GetCurrentFolderName) (Variables|Default|GetCurrentBoardName)))
          (Utilities|FlowControl|Sequence
            (:then_0
              (if (and _found (Utilities|Enum|Equal(Enum) _boardstate "NewEnumerator1"))
                (if (Class|BlueprintPathsLibrary|FileExists _path)
                  (Class|BlueprintFileUtilsBPLibrary|DeleteFile _path false false))))
            (:then_1
              (Default|AddBoardState _gi_ref (Variables|Default|GetCurrentFolderName) (Variables|Default|GetCurrentBoardName) "NewEnumerator2"))))
        (:else)))
    (:else)))

(event Custom|OnCellPressedEvent
  (params (RowIdx :type Integer) (ColIdx :type Integer) (EffectingButton :type Key%20Structure :default "None"))
  ;[1 1 1] Input related event
  (if (Math|Boolean|ANDBoolean (>= RowIdx 0) (>= ColIdx 0) (not (Variables|UserInteraction|GetMousePressed)))
    (bind _output_get (Variables|UserInteraction|SetPressedCell (Utilities|Struct|MakeST_Coord ColIdx RowIdx)))
    (Variables|UserInteraction|SetHoveringCell _output_get)
    (Variables|UserInteraction|SetMousePressed true)
    (CallFunction|SetupCellPreview EffectingButton)))

(event Custom|OnResetBoardProgress
  (CallFunction|ResetPuzzleProgress))

(event Custom|OnUserPuzzleSelected
  (params (EncodedInfo :type String) (BoardImage :type Texture%202D%20Dynamic%20Object%20Reference) (PuzzleHash :type String) (PuzzleName :type Text))
  (CallFunction|LoadUserBoard EncodedInfo PuzzleHash PuzzleName)
  (Variables|Default|SetCurrentBoardTextureDynamic BoardImage)
  (Variables|Default|SetbIsUserPuzzle true))

(event EventBeginPlay
  (bind _returnvalue (Game|GetPlatformName))
  (Utilities|FlowControl|Sequence
    (:then_0
      (bind _returnvalue_2 (Game|ConstructObjectfromClass "/Script/Nonogram.BoardManager"))
      (bind _output_get (Variables|Default|SetBoardManager_Ref _returnvalue_2))
      (Variables|/Script/Nonogram.BoardManager|SetGameMode _output_get self)
      (EventDispatchers|BindEventtoBoardClearedSignature _output_get (EventDispatchers|CreateEvent :!event Custom|OnBoardCompleteEvent))
      (bind _returnvalue_3 (Game|ConstructObjectfromClass (Variables|Default|GetBoardManager_Ref) "/Script/Nonogram.PlayLogger"))
      (Variables|/Script/Nonogram.BoardManager|SetLogger (Variables|Default|GetBoardManager_Ref) _returnvalue_3)
      (bind _returnvalue_4 (Game|AddComponentbyClass "/Game/_Game/Blueprints/BP_UI_Manager.BP_UI_Manager_C"))
      (Variables|Default|SetUI_Manager _returnvalue_4))
    (:then_1
      (bind _asgi_nonogram (Utilities|Casting|CastToGI_Nonogram (Game|GetGameInstance)))
      (Variables|Default|SetGI_Ref _asgi_nonogram))
    (:then_3
      (bind _returnvalue_5 (Game|ConstructObjectfromClass "/Script/Nonogram.ImageMaker"))
      (bind _boardmanager_ref (Variables|Default|GetBoardManager_Ref)
        (:then
          (Variables|/Script/Nonogram.BoardManager|SetImageMaker _boardmanager_ref _returnvalue_5))
        (:else)))
    (:then_4
      (Variables|UserInteraction|SetIsMobilePlatform (or (Utilities|Enum|Equal(Enum) _returnvalue "Android") (Utilities|Enum|Equal(Enum) _returnvalue "iOS"))))
    (:then_5
      (bind _gi_ref (Variables|Default|GetGI_Ref)
        (:then
          (Default|ApplySetting _gi_ref))
        (:else)))))

(event EventTick
  (params (DeltaSeconds :type Float%20%28single-precision%29)))

(fn ConstructionScript)

(fn ClickMultipleCell
  (bind _st_coord (Utilities|Struct|MakeST_Coord -1 -1))
  (Utilities|FlowControl|Sequence
    (:then_1
      ;[1 1 1] BoardManager에서 사용하는 자료형에 맞게 변경.
      (for _array_element (.CellCoords (CallFunction|GetDraggingCells (Variables|UserInteraction|GetPressedCell) (Variables|UserInteraction|GetReleasedCell)))
        (Utilities|Array|Add (LocalVariables|GetCells) (Math|Vector2D|MakeVector2D (Math|Conversions|ToFloat(Integer) (.x _array_element)) (Math|Conversions|ToFloat(Integer) (.y _array_element))))))
    (:then_2
      (bind _boardmanager_ref (Variables|Default|GetBoardManager_Ref)
        (:then
          (Class|BoardManager|ClickMultipleCells _boardmanager_ref (LocalVariables|GetCells) (Variables|UserInteraction|GetClickMode_Current)))
        (:else)))
    (:then_3
      (Variables|UserInteraction|SetPressedCell _st_coord)
      (Variables|UserInteraction|SetReleasedCell _st_coord)
      (Utilities|Array|Clear (Variables|UserInteraction|GetPreviewingCells))
      (Variables|UserInteraction|SetClickMode_Current "ECM_None"))))

(fn PreviewCells
  (bind _pressedcell (Variables|UserInteraction|GetPressedCell))
  (bind _hoveringcell (Variables|UserInteraction|GetHoveringCell))
  (bind (_cellcoords _ishorizontal) (CallFunction|GetDraggingCells _pressedcell _hoveringcell))
  (bind _returnvalue (not _ishorizontal))
  (Utilities|FlowControl|Sequence
    (:then_0
      (CallFunction|StopPreviewCells))
    (:then_2
      (CallFunction|PreviewCrossingCells))
    (:then_3
      (bind _output_get (Variables|UserInteraction|SetPreviewingCells _cellcoords))
      (for (_array_element _array_index) _output_get
        (bind _ui_manager (Variables|Default|GetUI_Manager)
          (:then
            (bind _wbp_play (Variables|/Game/_Game/Blueprints/BP_UI_Manager.BP_UI_Manager_C|GetWBP_Play _ui_manager)
              (:then
                (bind _wbp_board (Variables|/Game/_Game/UI/Board/WBP_Play.WBP_Play_C|GetWBP_Board _wbp_play)
                  (:then
                    (bind (_isvalid _wbp_cell) (Default|GetCellWidgetat _wbp_board (.X (Utilities|Struct|BreakST_Coord _array_element)) (.Y (Utilities|Struct|BreakST_Coord _array_element))))
                    (if _isvalid
                      (Default|OnSelected _wbp_cell (or _returnvalue (== _array_index 0)) (or _returnvalue (== _array_index (Utilities|Array|LastIndex (Variables|UserInteraction|GetPreviewingCells)))) (or _ishorizontal (== _array_index 0)) (or _ishorizontal (== _array_index (Utilities|Array|LastIndex (Variables|UserInteraction|GetPreviewingCells)))))))
                  (:else)))
              (:else)))
          (:else))))))

(fn GetDraggingCells
  (params (Start :type ST%20Coord%20Structure) (End :type ST%20Coord%20Structure))
  (Utilities|FlowControl|Sequence
    (:then_0
      (LocalVariables|SetHorizontalLength (Math|Integer|Absolute(Integer) (- (.x Start) (.x End))))
      (LocalVariables|SetVerticalLegnth (Math|Integer|Absolute(Integer) (- (.y Start) (.y End)))))
    (:then_1
      (if (> (LocalVariables|GetHorizontalLength) (LocalVariables|GetVerticalLegnth))
        (for _index (range (Math|Integer|Min(Integer) (.x Start) (.x End)) (Math|Integer|Max(Integer) (.x Start) (.x End)))
          (Utilities|Array|Add (LocalVariables|GetRetVal) (Utilities|Struct|MakeST_Coord _index (.y Start)))
          (LocalVariables|SetHorizontal true))
        (else
          (for _index_2 (range (Math|Integer|Min(Integer) (.y Start) (.y End)) (Math|Integer|Max(Integer) (.y Start) (.y End)))
            (Utilities|Array|Add (LocalVariables|GetRetVal) (Utilities|Struct|MakeST_Coord (.x Start) _index_2))
            (LocalVariables|SetHorizontal false)))))
    (:then_2
      (return (LocalVariables|GetRetVal) (LocalVariables|GetHorizontal)))))

(fn EqualCellStateClickMode
  (params (CellState :type ECellState%20Enum :default "ECS_Blank") (ClickMode :type EClickMode%20Enum :default "ECM_Blank"))
  (return (Utilities|Enum|Equal(Enum) CellState (Class|NonogramStatics|ClickModetoCellState ClickMode))))

(fn SetupCellPreview
  (params (EffectingButton :type Key%20Structure :default "None"))
  (bind _pressedcell (Variables|UserInteraction|GetPressedCell))
  (Utilities|FlowControl|Sequence
    (:then_0
      (bind _boardmanager_ref (Variables|Default|GetBoardManager_Ref)
        (:then
          (if (Utilities|Enum|Equal(Enum) "EBM_Play" (Class|BoardManager|GetBoardMode _boardmanager_ref))
            ;[1 1 1] 마우스 사용 시, 마우스 우클릭은 Not으로 변경.
            (Variables|UserInteraction|SetClickMode_Current (select (and (Class|KismetInputLibrary|KeyIsMouseButton EffectingButton) (== EffectingButton "RightMouseButton")) "ECM_Not" (Variables|Default|GetClickMode)))
            (else
              (Variables|UserInteraction|SetClickMode_Current "ECM_Fill")))
          ;[1 1 1] Press된 Cell이 무언가로 이미 채워져있다면 Blank모드로 변경.
          (bind _boardmanager_ref_2 (Variables|Default|GetBoardManager_Ref)
            (:then
              (if (not (CallFunction|EqualCellStateClickMode (Class|BoardManager|GetCellStateat _boardmanager_ref_2 (.x _pressedcell) (.y _pressedcell)) "ECM_Blank"))
                (Variables|UserInteraction|SetClickMode_Current "ECM_Blank")))
            (:else)))
        (:else)))
    (:then_1
      (Utilities|Array|Clear (Variables|UserInteraction|GetPreviewingCells)))
    (:then_2
      (CallFunction|PreviewCells))))

(fn StopPreviewCells
  (Utilities|FlowControl|Sequence
    (:then_0
      (for _array_element (Variables|UserInteraction|GetPreviewingCells)
        (bind _ui_manager (Variables|Default|GetUI_Manager)
          (:then
            (bind _wbp_play (Variables|/Game/_Game/Blueprints/BP_UI_Manager.BP_UI_Manager_C|GetWBP_Play _ui_manager)
              (:then
                (bind _wbp_board (Variables|/Game/_Game/UI/Board/WBP_Play.WBP_Play_C|GetWBP_Board _wbp_play)
                  (:then
                    (bind (_isvalid _wbp_cell) (Default|GetCellWidgetat _wbp_board (.X (Utilities|Struct|BreakST_Coord _array_element)) (.Y (Utilities|Struct|BreakST_Coord _array_element))))
                    (if _isvalid
                      (Default|OnSelectStopped _wbp_cell)))
                  (:else)))
              (:else)))
          (:else)))
      (Utilities|Array|Clear (Variables|UserInteraction|GetPreviewingCells)))))

(fn GetCrossCells
  (params (CenterX :type Integer) (CenterY :type Integer))
  (bind _boardmanager_ref (Variables|Default|GetBoardManager_Ref))
  (bind _returnvalue (Class|BoardManager|GetBoardInfo _boardmanager_ref))
  (bind (_displaytext _rownum _colnum) (Utilities|Struct|BreakBoardInfo _returnvalue))
  (Utilities|IsValid (Variables|Default|GetBoardManager_Ref)
    (:Is%20Valid
      (Utilities|FlowControl|Sequence
        (:then_0
          (LocalVariables|SetRowSize _rownum)
          (LocalVariables|SetColSize _colnum))
        (:then_1
          (for _index (range 0 (- (LocalVariables|GetRowSize) 1))
            (Utilities|Array|Add (LocalVariables|GetRetVal) (Utilities|Struct|MakeST_Coord CenterX _index))))
        (:then_2
          (for _index_2 (range 0 (- (LocalVariables|GetColSize) 1))
            (Utilities|Array|Add (LocalVariables|GetRetVal) (Utilities|Struct|MakeST_Coord _index_2 CenterY))))
        (:then_3
          (return (LocalVariables|GetRetVal)))))))

(fn PreviewCrossingCells
  (bind _hoveringcell (Variables|UserInteraction|GetHoveringCell))
  (Utilities|FlowControl|Sequence
    (:then_0
      (CallFunction|StopPreviewCrossingCells))
    (:then_1
      (bind _output_get (Variables|UserInteraction|SetCrossingCells (CallFunction|GetCrossCells (.x _hoveringcell) (.y _hoveringcell))))
      (for _array_element _output_get
        (bind _ui_manager (Variables|Default|GetUI_Manager)
          (:then
            (bind _wbp_play (Variables|/Game/_Game/Blueprints/BP_UI_Manager.BP_UI_Manager_C|GetWBP_Play _ui_manager)
              (:then
                (bind _wbp_board (Variables|/Game/_Game/UI/Board/WBP_Play.WBP_Play_C|GetWBP_Board _wbp_play)
                  (:then
                    (bind (_isvalid _wbp_cell) (Default|GetCellWidgetat _wbp_board (.X (Utilities|Struct|BreakST_Coord _array_element)) (.Y (Utilities|Struct|BreakST_Coord _array_element))))
                    (if _isvalid
                      (Default|StartCross _wbp_cell)))
                  (:else)))
              (:else)))
          (:else))))))

(fn StopPreviewCrossingCells
  (for _array_element (Variables|UserInteraction|GetCrossingCells)
    (bind _ui_manager (Variables|Default|GetUI_Manager)
      (:then
        (bind _wbp_play (Variables|/Game/_Game/Blueprints/BP_UI_Manager.BP_UI_Manager_C|GetWBP_Play _ui_manager)
          (:then
            (bind _wbp_board (Variables|/Game/_Game/UI/Board/WBP_Play.WBP_Play_C|GetWBP_Board _wbp_play)
              (:then
                (bind (_isvalid _wbp_cell) (Default|GetCellWidgetat _wbp_board (.X (Utilities|Struct|BreakST_Coord _array_element)) (.Y (Utilities|Struct|BreakST_Coord _array_element))))
                (if _isvalid
                  (Default|StopCross _wbp_cell)))
              (:else)))
          (:else)))
      (:else)))
  (Utilities|Array|Clear (Variables|UserInteraction|GetCrossingCells)))

(fn GetPlayTime
  (bind _output_get (LocalVariables|SetPlayTime (- (Utilities|Time|GetTimeSeconds) (Variables|Default|GetTime))))
  (bind _output_get_2 (LocalVariables|SetTime_Integer (Math|Float|Floor _output_get)))
  (return (LocalVariables|GetPlayTime) (/ _output_get_2 60) (Math|Integer|%(Integer) _output_get_2 60)))

(fn Undo
  (bind _boardmanager_ref (Variables|Default|GetBoardManager_Ref)
    (:then
      (bind _returnvalue (Class|BoardManager|Undo _boardmanager_ref))
      (if (not _returnvalue)
        (Development|PrintString "Undo Fail" true true "(R=1.000000,G=0.057999,B=0.000000,A=1.000000)")))
    (:else)))

(fn Redo
  (bind _boardmanager_ref (Variables|Default|GetBoardManager_Ref)
    (:then
      (bind _returnvalue (Class|BoardManager|Redo _boardmanager_ref))
      (if (not _returnvalue)
        (Development|PrintString "Redo Fail" true true "(R=1.000000,G=0.057999,B=0.000000,A=1.000000)")))
    (:else)))

(fn GetBoardInfo
  (params (FolderName :type Name) (BoardName :type Name))
  (bind (_found _boardinfo) (Default|GetBoardInfo (Variables|Default|GetGI_Ref) FolderName BoardName))
  (if _found
    (bind _boardmanager_ref (Variables|Default|GetBoardManager_Ref)
      (:then
        (Class|BoardManager|SetBoardInfo _boardmanager_ref _boardinfo)
        (return _found _boardinfo))
      (:else))
    (else
      (return false ""))))

(fn GetBoardMakerInfo
  (params (RowSize :type Integer) (ColSize :type Integer))
  (bind _returnvalue (Class|BoardManager|SetBoardMaker (Variables|Default|GetBoardManager_Ref) RowSize ColSize))
  (return _returnvalue))

(fn EmptyBoard
  (CallFunction|SaveBoardProgress)
  (bind _boardmanager_ref (Variables|Default|GetBoardManager_Ref)
    (:then
      (Class|BoardManager|ClearBoard _boardmanager_ref))
    (:else)))

(fn SaveBoardProgress
  (bind _boardmanager_ref (Variables|Default|GetBoardManager_Ref))
  (bind _boardmanager_ref_2 (Variables|Default|GetBoardManager_Ref))
  (bind _boardmanager_ref_3 (Variables|Default|GetBoardManager_Ref))
  (bind _returnvalue (Class|BoardManager|GetBoardMode _boardmanager_ref_3))
  (if (or (Utilities|Enum|Equal(Enum) "EBM_Play" _returnvalue) (Utilities|Enum|Equal(Enum) "EBM_User" _returnvalue))
    ;[1 1 1] 이미 완료한 퍼즐인지 확인
    (bind _gi_ref (Variables|Default|GetGI_Ref)
      (:then
        (bind (_found _boardstate) (Default|GetBoardState _gi_ref (Variables|Default|GetCurrentFolderName) (Variables|Default|GetCurrentBoardName)))
        (if (or (not _found) (and _found (not (Utilities|Enum|Equal(Enum) _boardstate "NewEnumerator2"))))
          (bind _boardmanager_ref_4 (Variables|Default|GetBoardManager_Ref)
            (:then
              (if (Class|BoardManager|GetBoardChanged _boardmanager_ref_4)
                (Default|AddBoardProgress (Variables|Default|GetGI_Ref) (Variables|Default|GetCurrentFolderName) (Variables|Default|GetCurrentBoardName) (Utilities|Struct|MakeST_BoardProgress (Class|BoardManager|GetCurrentMatchCount _boardmanager_ref) (Class|BoardManager|GetInfoCount _boardmanager_ref) (Class|BoardManager|GetEncodedBoard _boardmanager_ref_4) (.Time (CallFunction|GetPlayTime))))
                (Default|AddBoardState (Variables|Default|GetGI_Ref) (Variables|Default|GetCurrentFolderName) (Variables|Default|GetCurrentBoardName) "NewEnumerator1")
                (Class|BoardManager|SaveinProgressImage (Variables|Default|GetBoardManager_Ref) (Class|BoardManager|GetEncodedBoard _boardmanager_ref_4) (Utilities|String|ToString(Name) (Variables|Default|GetCurrentFolderName)) (Utilities|String|ToString(Name) (Variables|Default|GetCurrentBoardName)) (Class|BoardManager|GetRowSize _boardmanager_ref_2) (Class|BoardManager|GetColSize _boardmanager_ref_2) 127)))
            (:else))))
      (:else))))

(fn LoadBoard
  (params (FolderName :type Name) (BoardName :type Name) (PuzzleDisplayName :type Text))
  (Utilities|FlowControl|Sequence
    (:then_0
      (Variables|Default|SetCurrentFolderName FolderName)
      (Variables|Default|SetCurrentBoardName BoardName)
      (Variables|Default|SetCurrentBoardDisplayName PuzzleDisplayName))
    (:then_1
      ;[1 1 1] Set Default Puzzle
      (bind (_found _boardinfo) (CallFunction|GetBoardInfo (Variables|Default|GetCurrentFolderName) (Variables|Default|GetCurrentBoardName)))
      (if _found
        (bind _ui_manager (Variables|Default|GetUI_Manager)
          (:then
            (Default|ShowPlay _ui_manager _boardinfo "EBM_Play")
            ;[1 1 1] 이전 기록이 있으면 불러와서 적용
            (bind _gi_ref (Variables|Default|GetGI_Ref)
              (:then
                (bind (_found_2 _boardstate) (Default|GetBoardState _gi_ref (Variables|Default|GetCurrentFolderName) (Variables|Default|GetCurrentBoardName)))
                (if (and _found_2 (Utilities|Enum|Equal(Enum) _boardstate "NewEnumerator1"))
                  (bind (_bfound _encodedboard _playtime) (Default|GetBoardProgress _gi_ref (Variables|Default|GetCurrentFolderName) (Variables|Default|GetCurrentBoardName)))
                  (if _bfound
                    (LocalVariables|SetPrevPlayTime _playtime)
                    (bind _boardmanager_ref (Variables|Default|GetBoardManager_Ref)
                      (:then
                        (Class|BoardManager|SetBoardwithEncodedData _boardmanager_ref _encodedboard))
                      (:else)))
                  (else
                    ;;[1 1 1] 퍼즐 진행상황 적용할때 CheckAll을 함. 이 경우는 진행상황이 없으므로 따로 CheckAll
                    (bind _boardmanager_ref_2 (Variables|Default|GetBoardManager_Ref :!label _label)
                      (:then
                        (Class|BoardManager|CheckAll _boardmanager_ref_2))
                      (:else)))))
              (:else
                (goto _label))))
          (:else))))
    (:then_2
      (Variables|Default|SetTime (- (Utilities|Time|GetTimeSeconds) (LocalVariables|GetPrevPlayTime))))))

(fn LoadUserBoard
  (params (EncodedHint :type String) (PuzzleHash :type String) (PuzzleDisplayName :type Text))
  (Utilities|FlowControl|Sequence
    (:then_0
      (Variables|Default|SetCurrentFolderName "UserPuzzle")
      (Variables|Default|SetCurrentBoardName (Utilities|String|StringToName PuzzleHash))
      (Variables|Default|SetCurrentBoardDisplayName PuzzleDisplayName))
    (:then_1
      (bind _outboardinfo (Class|NonogramStatics|DecodeInfo EncodedHint))
      (bind _boardmanager_ref (Variables|Default|GetBoardManager_Ref)
        (:then
          (Class|BoardManager|SetBoardInfo _boardmanager_ref _outboardinfo)
          (bind _ui_manager (Variables|Default|GetUI_Manager)
            (:then
              (Default|ShowPlay _ui_manager _outboardinfo "EBM_User")
              ;[1 1 1] 이전 기록이 있으면 불러와서 적용
              (bind _gi_ref (Variables|Default|GetGI_Ref)
                (:then
                  (bind (_found _boardstate) (Default|GetBoardState _gi_ref (Variables|Default|GetCurrentFolderName) (Variables|Default|GetCurrentBoardName)))
                  (if (and _found (Utilities|Enum|Equal(Enum) _boardstate "NewEnumerator1"))
                    (bind (_bfound _encodedboard _playtime) (Default|GetBoardProgress _gi_ref (Variables|Default|GetCurrentFolderName) (Variables|Default|GetCurrentBoardName)))
                    (if _bfound
                      (LocalVariables|SetPrevPlayTime _playtime)
                      (bind _boardmanager_ref_2 (Variables|Default|GetBoardManager_Ref)
                        (:then
                          (Class|BoardManager|SetBoardwithEncodedData _boardmanager_ref_2 _encodedboard))
                        (:else)))
                    (else
                      ;;[1 1 1] 퍼즐 진행상황 적용할때 CheckAll을 함. 이 경우는 진행상황이 없으므로 따로 CheckAll
                      (bind _boardmanager_ref_3 (Variables|Default|GetBoardManager_Ref :!label _label)
                        (:then
                          (Class|BoardManager|CheckAll _boardmanager_ref_3))
                        (:else)))))
                (:else
                  (goto _label))))
            (:else)))
        (:else)))
    (:then_2
      (Variables|Default|SetTime (- (Utilities|Time|GetTimeSeconds) (LocalVariables|GetPrevPlayTime))))))

(fn ResetPuzzleProgress
  (bind _savedimgdir (CallFunction|GetSavedImgDir))
  (bind _savedimgdir_2 (CallFunction|GetSavedImgDir))
  (Utilities|FlowControl|Sequence
    (:then_0
      (bind _gi_ref (Variables|Default|GetGI_Ref)
        (:then
          (Default|ResetBoardState _gi_ref))
        (:else)))
    (:then_1
      (bind _ui_manager (Variables|Default|GetUI_Manager)
        (:then
          (Default|OnPuzzleProgressResetted _ui_manager))
        (:else)))
    (:then_2
      (if (Utilities|Paths|DirectoryExists _savedimgdir_2)
        (bind (_foundpaths _returnvalue) (Class|BlueprintFileUtilsBPLibrary|FindRecursive _savedimgdir_2 "" true false))
        (if _returnvalue
          (for _array_element _foundpaths
            (Class|BlueprintFileUtilsBPLibrary|DeleteFile _array_element false false)))))
    (:then_3
      (if (Utilities|Paths|DirectoryExists _savedimgdir)
        (bind (_foundpaths_2 _returnvalue_2) (Class|BlueprintFileUtilsBPLibrary|FindRecursive _savedimgdir "" false true))
        (if _returnvalue_2
          (for _array_element_2 _foundpaths_2
            (Class|BlueprintFileUtilsBPLibrary|DeleteDirectory _array_element_2 false false)))))))